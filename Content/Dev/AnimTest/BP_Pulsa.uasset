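; BP_Pulsa is an interactable whale test actor that the player's VR whale-watcher pawn can bring in for inspection.
; On Interact, if the pawn is not already inspecting, it registers itself as the inspection target and sets both inspection flags.
; It calls RootOn on the Pulsan mesh's animation Blueprint, then teleports to the pawn's BlueWhalePos transform.
; Interacting during an active inspection does nothing, as that branch is empty.
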(event `/Game/Gameplay/BPI_Interaction.Interact`
  (bind _ashmdloco_pawn_whale_watcher (cast `/Game/Characters/Player/HMDLocoPawn_WhaleWatcher` (`GameplayStatics.GetPlayerPawn` 0) :!pure true))
  (bind _bluewhalepos (`/Game/Characters/Player/HMDLocoPawn_WhaleWatcher.BlueWhalePos` _ashmdloco_pawn_whale_watcher))
  (if (`/Game/Characters/Player/HMDLocoPawn_WhaleWatcher.IsInspectingWhale` _ashmdloco_pawn_whale_watcher)
    (if (== (`/Game/Characters/Player/HMDLocoPawn_WhaleWatcher.InspectionTarget` _ashmdloco_pawn_whale_watcher) self)
      _)
    (else
      (set `self.IsBeingInspected` true)
      (set `/Game/Characters/Player/HMDLocoPawn_WhaleWatcher.InspectionTarget` self _ashmdloco_pawn_whale_watcher)
      (bind _asabp_whale_animation_test (cast `/Game/Dev/AnimTest/ABP_whaleAnimationTest` (`SkeletalMeshComponent.GetAnimInstance` (`self.Pulsan`))))
      (`/Game/Dev/AnimTest/ABP_whaleAnimationTest.RootOn` _asabp_whale_animation_test)
      (`self.K2_TeleportTo` (`SceneComponent.K2_GetComponentLocation` _bluewhalepos) (`SceneComponent.K2_GetComponentRotation` _bluewhalepos))
      (set `/Game/Characters/Player/HMDLocoPawn_WhaleWatcher.IsInspectingWhale` true _ashmdloco_pawn_whale_watcher))))

(fn `UserConstructionScript`)