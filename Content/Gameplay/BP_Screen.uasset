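; BP_Screen is a curved screen actor that unfolds through animation, then plays a whale ad video that can be paused.
; Both meshes start hidden; five seconds after BeginPlay the skeletal mesh appears, its ABP_Screen play rate is set, and an opening sound plays.
; PlayAd swaps the animated skeletal mesh for a static mesh with query-only collision and opens the ad in the media player.
; Interact alternates between pausing and resuming playback.
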(event `self.ReceiveBeginPlay`
  (bind _sk_curvedscreen_v02 (`self.SK_CurvedScreen_V02`))
  (`KismetSystemLibrary.Delay` 5.0)
  (set `/Game/Environment/Screen/ABP_Screen.ScreenAnimPlayRate` 1.0 (cast `/Game/Environment/Screen/ABP_Screen` (`SkeletalMeshComponent.GetAnimInstance` _sk_curvedscreen_v02) :!pure true))
  (`SceneComponent.SetVisibility` _sk_curvedscreen_v02 true false)
  (`AudioComponent.Play` (`self.OpeningSound`) 0.0))

(event `PlayAd`
  (bind _sm_curvedscreen_v02 (`self.SM_CurvedScreen_V02`))
  (bind _sk_curvedscreen_v02 (`self.SK_CurvedScreen_V02`))
  (`ActorComponent.SetActive` _sm_curvedscreen_v02 true false)
  (`SceneComponent.SetVisibility` _sm_curvedscreen_v02 true false)
  (`PrimitiveComponent.SetCollisionEnabled` _sm_curvedscreen_v02 "QueryOnly")
  (`ActorComponent.SetActive` _sk_curvedscreen_v02 false false)
  (`SceneComponent.SetVisibility` _sk_curvedscreen_v02 false false)
  (`MediaPlayer.OpenSource` (`self.WhaleAdPlayer`) "/Game/Movies/WhaleAd.WhaleAd"))

(event `/Game/Gameplay/BPI_Interaction.Interact`
  (bind _whaleadplayer (`self.WhaleAdPlayer`))
  (bind _isa (`/Engine/EditorBlueprintResources/StandardMacros.FlipFlop`)
    (:`A`
      (`MediaPlayer.Pause` _whaleadplayer))
    (:`B`
      (`MediaPlayer.Play` _whaleadplayer))))

(event `InputAction|GearPause`
  (params (Key :type "Key Structure" :default "AnyKey")))

(fn `UserConstructionScript`
  (bind _sm_curvedscreen_v02 (`self.SM_CurvedScreen_V02`))
  (`ActorComponent.SetActive` _sm_curvedscreen_v02 false false)
  (`SceneComponent.SetVisibility` _sm_curvedscreen_v02 false false)
  (`PrimitiveComponent.SetCollisionEnabled` _sm_curvedscreen_v02 "NoCollision")
  (`SceneComponent.SetVisibility` (`self.SK_CurvedScreen_V02`) false false))